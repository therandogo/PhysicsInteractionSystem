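; Actor component that lets its owning character hover, pick up, inspect and drop actors carrying a BPC_InteractableComponent.
; A looping timer line-traces from the owner's camera to track the focused interactable, which Interact hands the physics handle and camera, or drops if already holding.
; A faster timer reads the movement component's floor to notify stood-on interactables and block new interactions while airborne.
; Holding applies the interactable's walk speed until release.
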(event Custom|InteractWithFocusedActor
  ;[0.1464 0.4073 0.1547] Interaction with Focussed Objects
  (CallFunction|Interact))

(event EventBeginPlay
  ;[0.1766 0.3096 0.33] Setting Initial Dependencies and Timers
  (CallFunction|SetOwnerAttributes)
  ;;[1 1 1] Timer for Interaction Raycast
  (Utilities|Time|SetTimerbyFunctionName 0 "InteractionRaycast" 0.1 true)
  ;;[1 1 1] Timer for Standing on Interacatble Object check
  (Utilities|Time|SetTimerbyFunctionName 0 "StandOnInteractableCheck" 0.01 true))

(fn InteractionRaycast
  (bind _ownercamera (Variables|Default|GetOwnerCamera))
  (bind _returnvalue (Transformation|GetWorldLocation _ownercamera))
  (bind (_outhit _returnvalue_2) (Collision|LineTraceByChannel _returnvalue (+ _returnvalue (* (Math|Vector|GetForwardVector _ownercamera) (Variables|InteractionSettings|GetInteractDistance))) "TraceTypeQuery1" false 0 "None"))
  ;[0.424 0.1673 0.3981] Raycast detects the hit actor, checks if it has a BPC_InteractableComponent, if true then sends an interface call for OnHoverCheck and fetches the BPC_InteracatbaleComponent. Else removes any refernce of previous in focus actors or BPC_InteractableComponents
  (if _returnvalue_2
    ;;[0.4421 0.824 0.743] Check for checking the change in focused actor
    (if (!= (Variables|FocusedActor|GetInFocusActor) (.HitActor (Collision|BreakHitResult _outhit)))
      ;;[0.4421 0.824 0.743 0.33] Checking for previous BPC_InteractableCompoonent Ref
      (bind _bpc_interacatable (Variables|Default|GetBPC_Interacatable)
        (:then
          ;;[0.7865 0.374 0.4038] Clearing HoverCheck and BPC_InteractableComponent when the newly hovered object is found and previous references still remain
          (Class|BPIInteraction|HoveredCheck(Message) _bpc_interacatable false)
          (Variables|Default|SetBPC_Interacatable 0))
        (:else
          _))
      ;;[0.2601 0.4698 0.2123 0.75] Setting InFocusActor, HoveredCheck and BPC_InteractableCOmponent references
      (Variables|FocusedActor|SetInFocusActor (.HitActor (Collision|BreakHitResult _outhit)))
      (Utilities|IsValid (Actor|GetComponentbyClass (.HitActor (Collision|BreakHitResult _outhit)) "/Game/InteractionSystem/Components/BPC_InteractableComponent.BPC_InteractableComponent_C")
        (:Is%20Valid
          (Class|BPIInteraction|HoveredCheck(Message) (Actor|GetComponentbyClass (.HitActor (Collision|BreakHitResult _outhit)) "/Game/InteractionSystem/Components/BPC_InteractableComponent.BPC_InteractableComponent_C") true)
          (Variables|Default|SetBPC_Interacatable (Actor|GetComponentbyClass (.HitActor (Collision|BreakHitResult _outhit)) "/Game/InteractionSystem/Components/BPC_InteractableComponent.BPC_InteractableComponent_C")))))
    (else
      ;;[0.7865 0.374 0.4038] Clearing HoverCheck, focused actor and BPC_Interactable when raycast returns Null
      (bind _bpc_interacatable_2 (Variables|Default|GetBPC_Interacatable)
        (:then
          (Class|BPIInteraction|HoveredCheck(Message) _bpc_interacatable_2 false)
          (Variables|FocusedActor|SetInFocusActor 0)
          (Variables|Default|SetBPC_Interacatable 0))
        (:else)))))

(fn SetOwnerAttributes
  (bind _output_get (Variables|Owner|SetOwnerActor (Components|GetOwner)))
  (Variables|Default|SetOwnerCamera (Actor|GetComponentbyClass _output_get "/Script/Engine.CameraComponent"))
  (Variables|Default|SetPhysicsHandler (Actor|GetComponentbyClass (Variables|Owner|GetOwnerActor) "/Script/Engine.PhysicsHandleComponent"))
  (Variables|Default|SetCharacterMovement (Actor|GetComponentbyClass (Variables|Owner|GetOwnerActor) "/Script/Engine.CharacterMovementComponent")))

(fn Interact
  ;[0.349 0.1897 0.1945 0.738] If already interacting with something then first drop it
  (if (Variables|InteractionSettings|GetIsHolding)
    (CallFunction|StopInteraction)
    (else
      ;[0.2438 0.449 0.2081] Check if player can interact and if BPC_InteractableComponent is valid and then call  OnInteract interface, along with setting the dependencies
      (if (Variables|InteractionSettings|GetCanInteract)
        (bind _bpc_interacatable (Variables|Default|GetBPC_Interacatable)
          (:then
            (if (Default|GetCanInteract _bpc_interacatable)
              (Class|BPIInteraction|OnInteract(Message) (Variables|Default|GetBPC_Interacatable) (Variables|Default|GetPhysicsHandler) (Variables|Default|GetOwnerCamera))
              (CallFunction|SetInteractionDependencies)))
          (:else))))))

(fn StopInteraction
  (Variables|FocusedActor|GetHeldActor
    (:then
      (Class|BPIInteraction|OnDrop(Message) (Variables|Default|GetInteractedComponent))
      (Variables|InteractionSettings|SetIsHolding false)
      (Variables|FocusedActor|SetHeldActor 0)
      (Variables|Default|SetInteractedComponent 0)
      (Variables|/Script/Engine.CharacterMovementComponent|SetMaxWalkSpeed (Variables|Default|GetCharacterMovement) (Variables|InteractionSettings|GetDefaultWalkingSpeed)))
    (:else)))

(fn Inspect
  (params (MouseXY :type Vector%202D%20Structure))
  (bind _bpc_interacatable (Variables|Default|GetBPC_Interacatable))
  ;[0.2042 0.4198 0.1994 0.741] Gets mouse delta from the posessed pawn class/BP and sends it to held object
  (Class|BPIInteraction|OnInspect(Message) _bpc_interacatable MouseXY)
  (return (and (Utilities|IsValid _bpc_interacatable) (Variables|InteractionSettings|GetIsHolding))))

(fn StopInspect
  (Class|BPIInteraction|StopInspect(Message) (Variables|Default|GetBPC_Interacatable)))

(fn StandonInteractableCheck
  (bind _charactermovement (Variables|Default|GetCharacterMovement))
  (bind _currentfloor (Variables|/Script/Engine.CharacterMovementComponent|GetCurrentFloor _charactermovement))
  (bind _hitresult (Utilities|Struct|BreakFindFloorResult _currentfloor))
  (bind (_bblockinghit _binitialoverlap _time _distance _location _impactpoint _normal _impactnormal _physmat _hitactor) (Collision|BreakHitResult _hitresult))
  (bind _returnvalue (Actor|GetComponentbyClass _hitactor "/Game/InteractionSystem/Components/BPC_InteractableComponent.BPC_InteractableComponent_C"))
  ;[0.2264 0.3656 0.3865 0.813] Checking if Possesed pawn is not airborne and allowing for interaction only then
  (if _bblockinghit
    (if (!= (Variables|StoodOnActor|GetStoodOnObject) _hitactor)
      (CallFunction|SetCanInteractWObjects true)
      (bind _stoodonbpcinteractable (Variables|Default|GetStoodOnBPCInteractable :!label _label)
        (:then
          ;[0.474 0.2315 0.2647 0.75] Clearing StoodOnObject and BPC_InteractableComponent reference if posessed pawn is not on object anymore
          (Class|BPIInteraction|StoodOff(Message) _stoodonbpcinteractable)
          (Variables|StoodOnActor|SetStoodOnObject 0)
          (Variables|Default|SetStoodOnBPCInteractable 0))
        (:else
          _))
      ;[0.3032 0.449 0.2607 0.753] Setting BPC_InteractabaleComponen, StoodOnActor refernces and StoodOn interface check
      (Utilities|IsValid _hitactor
        (:Is%20Valid
          (if (Utilities|IsValid _returnvalue)
            (Class|BPIInteraction|Stoodon(Message) _returnvalue)
            (Variables|StoodOnActor|SetStoodOnObject _hitactor)
            (Variables|Default|SetStoodOnBPCInteractable _returnvalue)))))
    (else
      (CallFunction|SetCanInteractWObjects false)
      (goto _label))))

(fn SetCanInteractWObjects
  (params (CanInteract :type Boolean))
  (Variables|InteractionSettings|SetCanInteract CanInteract))

(fn SetInteractionDependencies
  (Variables|InteractionSettings|SetIsHolding true)
  (Variables|FocusedActor|SetHeldActor (Variables|FocusedActor|GetInFocusActor))
  (Variables|Default|SetInteractedComponent (Variables|Default|GetBPC_Interacatable))
  (Variables|/Script/Engine.CharacterMovementComponent|SetMaxWalkSpeed (Variables|Default|GetCharacterMovement) (Variables|/Game/InteractionSystem/Components/BPC_InteractableComponent.BPC_InteractableComponent_C|GetWalkingSpeedValue (Variables|Default|GetBPC_Interacatable))))