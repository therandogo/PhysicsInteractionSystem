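; Actor component that lets the owner's static mesh be highlighted, grabbed, carried and inspected by the player.
; Hover toggles custom depth; while held, Tick moves a physics handle target in front of the camera and applies mouse rotation during inspection.
; When stood on, it blocks interaction and a looping downward trace toggles physics and notifies the supporting interactable below.
; Stepping off restores interaction and physics, notifying that supporter.
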(event EventOnInteract
  (params (PhysicsHandler :type Physics%20Handle%20Component%20Object%20Reference) (CameraComponent :type Camera%20Component%20Object%20Reference))
  ;[0.3948 0.3948 0.3948] Interact
  (if (Variables|ObjectState|GetCanInteract)
    (CallFunction|OnInteraction PhysicsHandler CameraComponent)))

(event EventTick
  (params (DeltaSeconds :type Float%20%28single-precision%29))
  (if (Variables|ObjectState|GetInInteraction)
    (CallFunction|InspectionHandlingWCamera)))

(event EventHoveredCheck
  (params (IsHovered :type Boolean))
  ;[0.253 0.3618 0.4406 0.717] Allows for the hover material to be put on the objects
  (CallFunction|OnHoverRenderPass IsHovered))

(event EventBeginPlay
  ;[0.3656 0.3656 0.3656] Setting owner attributes
  (CallFunction|SetOwnerAttributes))

(event EventOnDrop
  ;[0.3948 0.3948 0.3948] Interact
  (CallFunction|OnStopInteraction))

(event EventOnInspect
  (params (MouseDelta :type Vector%202D%20Structure))
  ;[0.4615 0.4615 0.4615] Inspect
  (Variables|MouseInput|SetMouse%20Delta MouseDelta)
  (Variables|ObjectState|SetInInspection true))

(event EventStopInspect
  ;[0.4615 0.4615 0.4615] Inspect
  (Variables|ObjectState|SetInInspection false))

(event EventStoodon
  ;[0.409 0.5585 0.6115] Setting the timer for checking for other interactable actor below the currently stood on actor
  (Variables|ObjectState|SetCanInteract false)
  (Variables|SupportingActor|SetSupportingActor 0)
  (bind _returnvalue (Utilities|Time|SetTimerbyFunctionName 0 "OnStoodOn" 0.01 true)))

(event EventStoodOff
  ;[1 0.4746 0.5767] Pausing Timer, clearing references, enabling physics simulation and calling an interface to notify player walking off
  (Variables|ObjectState|SetCanInteract true)
  (Physics|SetSimulatePhysics (Variables|Default|GetOwnerStaticMesh) true)
  (Utilities|Time|PauseTimerbyHandle (stale EventStoodon _returnvalue))
  (bind _supportingactor (Variables|SupportingActor|GetSupportingActor)
    (:then
      (Class|BPIInteraction|StoodOff(Message) (Actor|GetComponentbyClass _supportingactor "BPC_InteractableComponent_C")))
    (:else)))

(fn SetOwnerAttributes
  (bind _output_get (Variables|Owner|SetOwnerActor (Components|GetOwner)))
  (Variables|Default|SetOwnerStaticMesh (Actor|GetComponentbyClass _output_get "/Script/Engine.StaticMeshComponent")))

(fn OnHoverRenderPass
  (params (bValue :type Boolean))
  (Rendering|SetRenderCustomDepth (Variables|Default|GetOwnerStaticMesh) bValue))

(fn OnInteraction
  (params (Physics%20Handler :type Physics%20Handle%20Component%20Object%20Reference) (Camera%20Component :type Camera%20Component%20Object%20Reference))
  (bind _ownerstaticmesh (Variables|Default|GetOwnerStaticMesh))
  (bind _ownerstaticmesh_2 (Variables|Default|GetOwnerStaticMesh))
  ;[0.262 0.4761 0.4948 0.648] Setting dependencies
  (Variables|Default|SetPhysics%20Handler Physics%20Handler)
  (Variables|Default|SetCamera%20Component Camera%20Component)
  ;[0.2179 0.4065 0.4448 0.617] Set location and rotation of held object to the grab component
  (Physics|Components|PhysicsHandle|GrabComponentatLocationwithRotation (Variables|Default|GetPhysics%20Handler) _ownerstaticmesh_2 "None" (Transformation|GetWorldLocation _ownerstaticmesh) (Transformation|GetWorldRotation _ownerstaticmesh))
  ;[0.7698 0.7259 0.464] Collision override in the actor itself to allow for custom collision rules
  (if (Variables|ObjectProperty|GetCollisionOverrideInActor)
    _
    (else
      (Collision|SetCollisionResponsetoChannel _ownerstaticmesh_2 "ECC_Pawn" "ECR_Ignore")))
  (Variables|ObjectState|SetInInteraction true))

(fn OnStopInteraction
  ;[0.5573 0.2655 0.2467 0.793] Clearing and resetting dependencies
  (Physics|Components|PhysicsHandle|ReleaseComponent (Variables|Default|GetPhysics%20Handler))
  (Variables|Default|SetPhysics%20Handler 0)
  (Variables|Default|SetCamera%20Component 0)
  (if (Variables|ObjectProperty|GetCollisionOverrideInActor)
    _
    (else
      (Collision|SetCollisionResponsetoChannel (Variables|Default|GetOwnerStaticMesh) "ECC_Pawn" "ECR_Block")))
  (Variables|ObjectState|SetInInteraction false))

(fn InspectionHandlingWCamera
  (bind _camera_component (Variables|Default|GetCamera%20Component))
  (bind _mouse_delta (Variables|MouseInput|GetMouse%20Delta))
  (bind (_x _y) (Math|Vector2D|BreakVector2D _mouse_delta))
  (Variables|Default|GetPhysics%20Handler
    (:then
      (Variables|Default|GetCamera%20Component
        (:then
          (Physics|Components|PhysicsHandle|SetTargetLocation (Variables|Default|GetPhysics%20Handler) (+ (Transformation|GetWorldLocation _camera_component) (* (Math|Vector|GetForwardVector _camera_component) (Variables|ObjectProperty|GetInteractOffsetValue))))
          (if (Variables|ObjectState|GetInInspection)
            (Class|PhysicsHandleComponent|SetTargetRotation (Variables|Default|GetPhysics%20Handler) (Math|Rotator|CombineRotators (.TargetRotation (Class|PhysicsHandleComponent|GetTargetLocationandRotation (Variables|Default|GetPhysics%20Handler))) (Math|Rotator|MakeRotator 0.0 _y _x)))))
        (:else)))
    (:else)))

(fn OnStoodon
  (bind _ownerstaticmesh (Variables|Default|GetOwnerStaticMesh))
  (bind _returnvalue (Transformation|GetWorldLocation _ownerstaticmesh))
  (bind (_outhit _returnvalue_2) (Collision|LineTraceByChannel _returnvalue (+ (* (Math|Vector|GetUpVector (Variables|/Script/Engine.Actor|GetRootComponent (Variables|Owner|GetOwnerActor))) (* (.z (Transformation|GetWorldScale (Variables|Default|GetOwnerStaticMesh))) (* -1.0 (Variables|ObjectProperty|GetActorBelowCheckLength)))) _returnvalue) "TraceTypeQuery1" false 0 "None"))
  (if _returnvalue_2
    (if (!= (.HitActor (Collision|BreakHitResult _outhit)) (Variables|SupportingActor|GetSupportingActor))
      (Physics|SetSimulatePhysics (Variables|Default|GetOwnerStaticMesh) false)
      (Utilities|IsValid (Actor|GetComponentbyClass (.HitActor (Collision|BreakHitResult _outhit)) "BPC_InteractableComponent_C")
        (:Is%20Valid
          (Class|BPIInteraction|Stoodon(Message) (Actor|GetComponentbyClass (.HitActor (Collision|BreakHitResult _outhit)) "BPC_InteractableComponent_C"))
          (Variables|SupportingActor|SetSupportingActor (.HitActor (Collision|BreakHitResult _outhit))))))
    (else
      (Physics|SetSimulatePhysics (Variables|Default|GetOwnerStaticMesh) true))))

(fn GetCanInteract
  (return (Variables|ObjectState|GetCanInteract)))